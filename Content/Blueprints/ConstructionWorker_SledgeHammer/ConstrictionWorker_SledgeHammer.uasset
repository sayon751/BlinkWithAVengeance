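; Sledgehammer construction worker AI pawn that chases an Explorer it sees and starts a randomized melee combo on reaching it.
; PawnSensing drives AIMoveTo into MeleeAttack, which sets Attack and rolls one to three swings, each with a random variant.
; ConstructionWorkerSledgeHammerInfo clears those values when the swing ends, but MeleeAttack's DoOnce is never reset.
; BeginPlay also registers the worker as a Team-sense stimuli source.
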(event OnSeePawn(PawnSensing)
  (params (Pawn :type Pawn%20Object%20Reference))
  (bind _asexplorer (Utilities|Casting|CastToExplorer Pawn))
  (AI|AIMoveTo self "0, 0, 0" _asexplorer 1e+01 true
    (:OnSuccess
      (CallFunction|MeleeAttack))))

(event Custom|MeleeAttack
  (bind _returnvalue (Math|Random|RandomIntegerinRange 1 5))
  (Utilities|FlowControl|DoOnce false
    (:Completed
      (Utilities|FlowControl|Sequence
        (:then_0
          (bind _output_get (Variables|Default|SetAttack true))
          (if _output_get
            (Variables|Default|SetSwingEnd false)))
        (:then_1
          (bind _output_get_2 (Variables|Default|SetNumberOfAttacks (Math|Random|RandomIntegerinRange 1 3))))
        (:then_2
          (switch int _output_get_2
            (:1
              (Variables|Default|SetFirstAttack _returnvalue))
            (:2
              (Variables|Default|SetFirstAttack _returnvalue)
              (Variables|Default|SetSecondAttack _returnvalue))
            (:3
              (Variables|Default|SetFirstAttack _returnvalue)
              (Variables|Default|SetSecondAttack _returnvalue)
              (Variables|Default|SetThirdAttack _returnvalue))))))))

(event EventBeginPlay
  (Class|AIPerceptionSystem|RegisterPerceptionStimuliSource "/Script/AIModule.AISense_Team" self))

(event Collision|EventActorBeginOverlap
  (params (OtherActor :type Actor%20Object%20Reference)))

(event EventTick
  (params (DeltaSeconds :type Float%20%28single-precision%29)))

(event EventConstructionWorkerSledgeHammerInfo
  (params (IsAttacking :type Boolean) (SwingEnd :type Boolean))
  (if SwingEnd
    (Variables|Default|SetSwingEnd SwingEnd)
    (Variables|Default|SetAttack (not SwingEnd))
    (switch int (Variables|Default|GetNumberOfAttacks)
      (:1
        (Variables|Default|SetFirstAttack 0))
      (:2
        (Variables|Default|SetFirstAttack 0)
        (Variables|Default|SetSecondAttack 0))
      (:3
        (Variables|Default|SetFirstAttack 0)
        (Variables|Default|SetSecondAttack 0)
        (Variables|Default|SetThirdAttack 0)))))

(fn ConstructionScript)